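; BP_FadeMesh is an actor with a static mesh that fades toward a configurable opacity on request and can fade back.
; The construction script assigns the chosen mesh and gives its first material slot a dynamic instance of FadeMaterial.
; StartFade plays FadeTimeline, which lowers the material's Opacity parameter from 1 toward EndingFadeAmount as FadeAmount rises, and EndFade reverses the same timeline.
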(event EventBeginPlay)

(event Collision|EventActorBeginOverlap
  (params (OtherActor :type Actor%20Object%20Reference)))

(event EventTick
  (params (DeltaSeconds :type Float%20%28single-precision%29)))

(event EventEndFade
  (bind _fadeamount (Timeline|FadeTimeline Reverse)
    (:Update
      (Rendering|Material|SetScalarParameterValue (Variables|Default|GetDynamicMaterial) "Opacity" (- 1.0 (* _fadeamount (- 1.0 (Variables|Default|GetEndingFadeAmount)))) :!class /Script/Engine.MaterialInstanceDynamic))))

(event EventStartFade
  (bind _fadeamount (Timeline|FadeTimeline Play)
    (:Update
      (Rendering|Material|SetScalarParameterValue (Variables|Default|GetDynamicMaterial) "Opacity" (- 1.0 (* _fadeamount (- 1.0 (Variables|Default|GetEndingFadeAmount)))) :!class /Script/Engine.MaterialInstanceDynamic))))

(fn ConstructionScript
  (Components|StaticMesh|SetStaticMesh (Variables|Default|GetStaticMesh) (Variables|Default|GetMeshToUse))
  (bind _returnvalue (Rendering|Material|CreateDynamicMaterialInstance (Variables|Default|GetFadeMaterial) "None" "None" :!class /Script/Engine.KismetMaterialLibrary))
  (bind _output_get (Variables|Default|SetDynamicMaterial _returnvalue))
  (Rendering|Material|SetMaterial (Variables|Default|GetStaticMesh) 0 _output_get))